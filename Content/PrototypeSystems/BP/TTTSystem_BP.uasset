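; Tic-tac-toe board system that builds a resizable, centered square grid of instanced tiles, from 3x3 to 10x10.
; Flat arrays hold each tile's transform, state and piece mesh, with helpers converting between index and grid coordinates.
; AddPiece spawns an X or O StaticMeshActor on an empty tile, and ResetPieces clears them.
; CheckWinner scans rows, columns and both diagonals for a full-length line, while IsGameTied tests for a full board.
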(event EventBeginPlay
  (CallFunction|UpdateGrid))

(fn ConstructionScript)

(fn UpdateGrid
  (bind _grid (Variables|Default|GetGrid))
  (bind _gridgap (Variables|Config|GetGridGap))
  (Utilities|Array|Clear (Variables|State|GetCurrentInstances))
  (Utilities|Array|Clear (Variables|Components|GetMeshes))
  (Utilities|Array|Clear (Variables|State|GetTileState))
  (Components|InstancedStaticMesh|ClearInstances _grid)
  (LocalVariables|SetGridOffsetVal (CallFunction|GetGridOffsetCenteringVal (Variables|Config|GetGridDimensions) (Variables|Config|GetGridGap)))
  (bind _output_get (LocalVariables|SetLastIndex (CallFunction|GetMainArraysLastIndex (Variables|Config|GetGridDimensions))))
  (for _index (range 0 _output_get)
    (Utilities|Array|Add (Variables|State|GetCurrentInstances) (Math|Transform|MakeTransform (Math|Vector|MakeVector (- (* (.X (CallFunction|GetGridCoordsfromIndex _index (Variables|Config|GetGridDimensions))) _gridgap) (LocalVariables|GetGridOffsetVal)) (- (* (.Y (CallFunction|GetGridCoordsfromIndex _index (Variables|Config|GetGridDimensions))) _gridgap) (LocalVariables|GetGridOffsetVal)) 0.0) "0, 0, 0" "1,1,1")))
  (Components|InstancedStaticMesh|AddInstances _grid (Variables|State|GetCurrentInstances) false)
  (for _index_2 (range 0 (LocalVariables|GetLastIndex))
    (Utilities|Array|Add (Variables|Components|GetMeshes) 0))
  (for _index_3 (range 0 (LocalVariables|GetLastIndex))
    (Utilities|Array|Add (Variables|State|GetTileState) "NewEnumerator0")))

(fn GetGridCoordsfromIndex
  (params (Index :type Integer) (GridDimensions :type Integer))
  (return (Math|Integer|%(Integer) Index GridDimensions) (/ Index GridDimensions)))

(fn GetIndexfromGridCoords
  (params (X :type Integer) (Y :type Integer) (GridDimensions :type Integer))
  (return (+ X (* Y GridDimensions))))

(fn GetGridOffsetCenteringVal
  (params (GridDimensions :type Integer) (GridGap :type Float%20%28single-precision%29))
  (return (/ (* (- GridDimensions 1) GridGap) 2.0)))

(fn AdjustGrid
  (params (IsIncrementing :type Boolean))
  (bind _output_get (Variables|Config|SetGridDimensions (Math|Integer|Clamp(Integer) (+ (stale _output_get) (Math|Integer|SelectInt 1 -1 IsIncrementing)) 3 10)))
  (CallFunction|UpdateGrid)
  (return _output_get))

(fn AddPiece
  (params (IsOPlayer :type Boolean) (LocationIndex :type Integer))
  (bind _tilestate (Variables|State|GetTileState))
  (if (Utilities|Enum|Equal(Enum) (Utilities|Array|Get(acopy) _tilestate LocationIndex) "NewEnumerator0")
    (Utilities|Array|SetArrayElem _tilestate LocationIndex (CallFunction|GetTileStatefromIsO IsOPlayer) true)
    (bind _returnvalue (Game|SpawnActorfromClass "/Script/Engine.StaticMeshActor" (Utilities|Array|Get(acopy) (Variables|State|GetCurrentInstances) LocationIndex) "Undefined" 0 0))
    (bind _output_get (LocalVariables|SetCurrentMesh _returnvalue))
    (Transformation|SetMobility _output_get "Movable")
    (Components|StaticMesh|SetStaticMesh (Variables|/Script/Engine.StaticMeshActor|GetStaticMeshComponent _output_get) (select IsOPlayer (Variables|Components|GetMeshO) (Variables|Components|GetMeshX)))
    (Utilities|Array|SetArrayElem (Variables|Components|GetMeshes) LocationIndex _output_get)
    (Math|Integer|IncrementInt (Variables|State|GetPieceCount)
      (:%20%20
        (return true)))
    (else
      (return false))))

(fn ResetPieces
  (bind _meshes (Variables|Components|GetMeshes))
  (bind _tilestate (Variables|State|GetTileState))
  (for (_array_element _array_index) _meshes
    (Utilities|IsValid _array_element
      (:Is%20Valid
        (Actor|DestroyActor _array_element)
        (Utilities|Array|SetArrayElem _meshes _array_index 0))))
  (Variables|State|SetPieceCount 0)
  (for (_ _array_index_2) _tilestate
    (Utilities|Array|SetArrayElem _tilestate _array_index_2 "NewEnumerator0")))

(fn GetTileStatefromIsO
  (params (IsO :type Boolean))
  (if IsO
    (return "NewEnumerator2")
    (else
      (return "NewEnumerator1"))))

(fn StartStopGame
  (params (IsStarting :type Boolean))
  (CallFunction|ResetPieces))

(fn CheckWinner
  (params (StartFromIndex :type Integer))
  (bind _griddimensions (Variables|Config|GetGridDimensions))
  (if (>= (Variables|State|GetPieceCount) (Variables|Config|GetGridDimensions))
    (LocalVariables|SetCompareTileState (Utilities|Array|Get(acopy) (Variables|State|GetTileState) StartFromIndex))
    (if (Math|Boolean|ORBoolean (CallFunction|ScanRoworColumn (LocalVariables|GetCompareTileState) _griddimensions false) (CallFunction|ScanRoworColumn (LocalVariables|GetCompareTileState) _griddimensions true) (CallFunction|ScanDiagonal (LocalVariables|GetCompareTileState) _griddimensions true) (CallFunction|ScanDiagonal (LocalVariables|GetCompareTileState) _griddimensions false))
      (return (LocalVariables|GetCompareTileState)))
    (else
      (return "NewEnumerator0"))))

(fn GetAdjacentTile
  (params (Index :type Integer) (GridDimensions :type Integer) (Direction :type TTTDirection%20Enum :default "NewEnumerator0"))
  (bind (_x _y) (CallFunction|GetGridCoordsfromIndex Index GridDimensions))
  (bind (_x_2 _y_2) (CallFunction|GetCoordAdderfromDirection Direction))
  (bind _returnvalue (- GridDimensions 1))
  (bind _returnvalue_2 (+ _x _x_2))
  (bind _returnvalue_3 (+ _y _y_2))
  (return (CallFunction|GetIndexfromGridCoords _returnvalue_2 _returnvalue_3 GridDimensions) (and (Math|Integer|InRange(Integer) _returnvalue_2 0 _returnvalue) (Math|Integer|InRange(Integer) _returnvalue_3 0 _returnvalue))))

(fn GetCoordAdderfromDirection
  (params (Direction :type TTTDirection%20Enum :default "NewEnumerator0"))
  (switch Utilities|FlowControl|Switch|SwitchonTTTDirection Direction
    (:NewEnumerator0
      (return 1 0))
    (:NewEnumerator1
      (return 1 1))
    (:NewEnumerator2
      (return 0 1))
    (:NewEnumerator3
      (return -1 1))
    (:NewEnumerator4
      (return -1 0))
    (:NewEnumerator5
      (return -1 -1))
    (:NewEnumerator6
      (return 0 -1))
    (:NewEnumerator7
      (return 1 -1))))

(fn GetMainArraysLastIndex
  (params (GridDimensions :type Integer))
  (return (- (* GridDimensions GridDimensions) 1)))

(fn GetMainArraysLength
  (params (GridDimensions :type Integer))
  (return (* GridDimensions GridDimensions)))

(fn ScanRoworColumn
  (params (CompareTileState :type TileState%20Enum :default "NewEnumerator0") (GridDimensions :type Integer) (IsRows :type Boolean))
  (bind _returnvalue (- GridDimensions 1))
  (bind _index (Utilities|FlowControl|ForLoopwithBreak 0 _returnvalue)
    (:LoopBody
      (LocalVariables|SetCurrentCount 0)
      (bind _index_2 (Utilities|FlowControl|ForLoopwithBreak 0 _returnvalue)
        (:LoopBody
          (if (Utilities|Enum|Equal(Enum) (Utilities|Array|Get(acopy) (Variables|State|GetTileState) (CallFunction|GetIndexfromGridCoords (Math|Integer|SelectInt _index _index_2 IsRows) (Math|Integer|SelectInt _index_2 _index IsRows) GridDimensions)) CompareTileState)
            (bind _result (Math|Integer|IncrementInt (LocalVariables|GetCurrentCount))
              (:%20%20
                (if (>= _result GridDimensions)
                  (return true))))))))))

(fn ScanDiagonal
  (params (CompareTileState :type TileState%20Enum :default "NewEnumerator0") (GridDimensions :type Integer) (IsReversed :type Boolean))
  (bind _returnvalue (- GridDimensions 1))
  (bind _index (Utilities|FlowControl|ForLoopwithBreak 0 _returnvalue)
    (:LoopBody
      (if (Utilities|Enum|Equal(Enum) (Utilities|Array|Get(acopy) (Variables|State|GetTileState) (CallFunction|GetIndexfromGridCoords (Math|Integer|SelectInt _index _index IsReversed) (Math|Integer|SelectInt (- _returnvalue _index) _index IsReversed) GridDimensions)) CompareTileState)
        (bind _result (Math|Integer|IncrementInt (LocalVariables|GetCurrentCount))
          (:%20%20
            (if (>= _result GridDimensions)
              (return true))))))))

(fn IsGameTied
  (return (>= (Variables|State|GetPieceCount) (CallFunction|GetMainArraysLength (Variables|Config|GetGridDimensions)))))