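; Player pawn for a two-player Tic-Tac-Toe prototype, handling mouse input, turn order, HUD and camera.
; Clicks trace from the cursor and use the hit item index as the tile index for the level's TTTSystem, which places pieces and checks winners.
; HUD events start or stop play and resize the grid, with camera height scaling to grid size.
; Wins are only printed; play continues.
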(event Custom|GameStartStop
  (bind _output_get (Variables|State|SetIsGameActive (not (stale _output_get))))
  (Default|SwitchIsPlaying (Variables|Components|GetHUD_UI) (Variables|State|GetIsGameActive) (Variables|State|GetIsCurrentlyOPlayer))
  (Default|StartStopGame (Variables|Components|GetTTTsystem) (Variables|State|GetIsGameActive))
  (Variables|State|SetIsCurrentlyOPlayer false))

(event Custom|GridAdjust
  (params (IsIncrementing :type Boolean))
  (bind _griddimensions (Default|AdjustGrid (Variables|Components|GetTTTsystem) IsIncrementing))
  (CallFunction|UpdateCamera _griddimensions 2.5e+02))

(event EventBeginPlay
  (CallFunction|InitUI)
  (CallFunction|InitSystem)
  (CallFunction|UpdateCamera 3 2.5e+02))

(event Collision|EventActorBeginOverlap
  (params (OtherActor :type Actor%20Object%20Reference)))

(event EventTick
  (params (DeltaSeconds :type Float%20%28single-precision%29)))

(event Input|ActionEvents|InputActionSelect
  (params (Key :type Key%20Structure :default "None"))
  (:Pressed
    (if (Variables|State|GetIsGameActive)
      (bind (_index _success) (CallFunction|ClickTraceforTile))
      (if _success
        (bind _success_2 (Default|AddPiece (Variables|Components|GetTTTsystem) (Variables|State|GetIsCurrentlyOPlayer) _index))
        (if _success_2
          (bind _state (Default|CheckWinner (Variables|Components|GetTTTsystem) _index))
          (switch Utilities|FlowControl|Switch|SwitchonTileState _state
            (:NewEnumerator0
              _)
            (:NewEnumerator1
              (Development|PrintString "X wins"))
            (:NewEnumerator2
              (Development|PrintString "O wins")))
          (bind _output_get (Variables|State|SetIsCurrentlyOPlayer (not (stale _output_get))))
          (Default|UpdateStatusTextCurrentPlayer (Variables|Components|GetHUD_UI) (Variables|State|GetIsCurrentlyOPlayer) true))))))

(fn ConstructionScript)

(fn InitUI
  (bind _returnvalue (Game|GetPlayerController 0))
  (bind _returnvalue_2 (UserInterface|CreateWidget "/Game/PrototypeSystems/UI/HUD_UI.HUD_UI_C"))
  (bind _output_get (Variables|Components|SetHUD_UI _returnvalue_2))
  (UserInterface|Viewport|AddtoViewport _output_get 0)
  (Variables|/Script/Engine.PlayerController|SetbShowMouseCursor _returnvalue true)
  (Input|SetInputModeGameandUI _returnvalue _output_get "DoNotLock" true)
  (EventDispatchers|BindEventtoOnGameStartStop _output_get (EventDispatchers|CreateEvent :!event Custom|GameStartStop))
  (EventDispatchers|BindEventtoOnGridAdjust _output_get (EventDispatchers|CreateEvent :!event Custom|GridAdjust)))

(fn ClickTraceforTile
  (bind _returnvalue (Game|GetPlayerController 0))
  (bind (_worldlocation _worlddirection _returnvalue_2) (Game|Player|ConvertMouseLocationToWorldSpace _returnvalue))
  (if _returnvalue_2
    (bind (_outhit _returnvalue_3) (Collision|LineTraceForObjects _worldlocation (+ _worldlocation (* _worlddirection 5e+03)) (Utilities|Array|MakeArray "ObjectTypeQuery7") false 0 "None"))
    (if _returnvalue_3
      (return (.HitItem (Collision|BreakHitResult _outhit)) true)
      (else
        _)))
  (return -1 false))

(fn InitSystem
  (bind _outactors (Actor|GetAllActorsOfClass "/Game/PrototypeSystems/BP/TTTSystem.TTTSystem_C"))
  (if (Utilities|Array|IsValidIndex _outactors)
    (Variables|Components|SetTTTsystem (Utilities|Array|Get(acopy) _outactors))))

(fn UpdateCamera
  (params (GridDimensions :type Integer) (DistanceMultiplier :type Float%20%28single-precision%29))
  (Transformation|SetRelativeLocation (Variables|Default|GetCamera) (Math|Vector|MakeVector 0.0 0.0 (* GridDimensions DistanceMultiplier)) false false))